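; Game mode Blueprint that lets the first player take control of one of two characters, MyCharacter or MyOtherCharacter.
; Two events, StartMyCharacter and StartMyOtherCharacter, each call a matching select function.
; Each function spawns its character class at a fixed point slightly above the world origin and has player controller 0 possess it.
; BeginPlay and Tick are unused, so selection happens only when one of those events is called.
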(event Custom|StartMyCharacter
  (CallFunction|SelectMyCharacter))

(event Custom|StartMyOtherCharacter
  (CallFunction|SelectMyOtherCharacter))

(event EventBeginPlay)

(event EventTick
  (params (DeltaSeconds :type Float%20%28single-precision%29)))

(fn ConstructionScript)

(fn SelectMyCharacter
  (bind _returnvalue (Game|SpawnActorfromClass "/Script/PrimeiroCodigo.MyCharacter" (Math|Transform|MakeTransform "0, 0,120.000000") "Undefined" 0 0))
  (Pawn|Possess (Game|GetPlayerController 0) _returnvalue))

(fn SelectMyOtherCharacter
  (bind _returnvalue (Game|SpawnActorfromClass "/Script/PrimeiroCodigo.MyOtherCharacter" (Math|Transform|MakeTransform "0, 0,120.000000") "Undefined" 0 0))
  (Pawn|Possess (Game|GetPlayerController 0) _returnvalue))